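; Player combat component for BP_ThirdPersonCharacter that handles target lock, sword combos, hit detection and dodging.
; Lock-on sphere-traces from the camera, attaches a marker, switches to controller-driven rotation and aims at the target each tick.
; Attack presses buffer a combo that montage notifies continue or stop, while Begin/EndDamageTrace toggle a timer-looped blade trace applying rate-limited damage.
; Dodge plays a directional montage from WASD under controller rotation, otherwise forward.
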(event Custom|Begin%20Damage%20Trace
  ;[0.05208 0.05208 0.05208] Sword Traces
  (bind _returnvalue (Utilities|Time|SetTimerbyEvent (delegate Custom|Damage%20Trace) 0.01 true)))

(event Custom|Damage%20Trace
  (bind _player_bp (Variables|Default|GetPlayer%20BP))
  ;[0.05208 0.05208 0.05208] Sword Traces
  ;;[0.05208 0.05208 0.05208] 검 히트박스 크기 변경 시 Radius 수정
  (bind (_outhit _returnvalue) (Collision|SphereTraceForObjects (Transformation|GetWorldLocation (Variables|/Game/ThirdPerson/Blueprints/BP_ThirdPersonCharacter.BP_ThirdPersonCharacter_C|GetStart%20Sword%20Trace%20Pos _player_bp)) (Transformation|GetWorldLocation (Variables|/Game/ThirdPerson/Blueprints/BP_ThirdPersonCharacter.BP_ThirdPersonCharacter_C|GetEnd%20Sword%20Trace%20Pos _player_bp)) 25.0 (Utilities|Array|MakeArray "ObjectTypeQuery3") false 0 "ForOneFrame"))
  (if _returnvalue
    (Utilities|FlowControl|DoOnce false :!label _label
      (:Completed
        (Game|Damage|ApplyDamage (.HitActor (Collision|BreakHitResult _outhit)) (Variables|Default|GetswordDamage) 0 0)
        (Utilities|FlowControl|Delay 0.3)
        (goto _label Reset)))))

(event Custom|End%20Damage%20Trace
  ;[0.05208 0.05208 0.05208] Sword Traces
  (if (Utilities|Time|IsValidTimerHandle (stale Custom|Begin%20Damage%20Trace _returnvalue))
    (Utilities|Time|ClearandInvalidateTimerbyHandle (stale Custom|Begin%20Damage%20Trace _returnvalue))))

(event Input|EnhancedActionEvents|EnhancedInputActionIA_Lock
  (params (ActionValue :type Boolean) (ElapsedSeconds :type Float%20%28double-precision%29) (TriggeredSeconds :type Float%20%28double-precision%29) (InputAction :type Input%20Action%20Object%20Reference :default "/Game/ThirdPerson/Input/Actions/IA_Lock.IA_Lock"))
  (bind _returnvalue (Game|GetPlayerCameraManager 0))
  (bind _player_bp (Variables|Default|GetPlayer%20BP))
  (bind _player_bp_2 (Variables|Default|GetPlayer%20BP))
  (bind _transformcomponent (Variables|/Script/Engine.PlayerCameraManager|GetTransformComponent _returnvalue))
  (bind _charactermovement (Variables|/Script/Engine.Character|GetCharacterMovement _player_bp))
  (bind _charactermovement_2 (Variables|/Script/Engine.Character|GetCharacterMovement _player_bp_2))
  (bind _returnvalue_2 (Transformation|GetWorldLocation _transformcomponent))
  ;[0.05208 0.05208 0.05208] Target Lock
  (:Started
    (Variables|Default|GetTarget%20Lock%20Actor
      (:then
        ;;[0.07292 0.07292 0.07292] 락온 해제 시 일반 움직임으로 변경
        (Variables|Default|SetTarget%20Lock%20Actor 0)
        (Variables|/Script/Engine.CharacterMovementComponent|SetbOrientRotationToMovement _charactermovement_2 true)
        (Variables|/Script/Engine.CharacterMovementComponent|SetbUseControllerDesiredRotation _charactermovement_2 false)
        ;;[0.07292 0.07292 0.07292] 락온 종료 시 아이콘 제거
        (Actor|DestroyActor (Variables|Default|GetTarget%20Lock%20Widget)))
      (:else
        (bind (_outhit _returnvalue_3) (Collision|SphereTraceForObjects "0, 0, 0" (+ (Math|Vector|MakeVector (.x _returnvalue_2) (.y _returnvalue_2) (+ (.z _returnvalue_2) 2e+01)) (* (Math|Vector|GetForwardVector (Transformation|GetWorldRotation _transformcomponent)) 1e+03)) 1.5e+02 (Utilities|Array|MakeArray "ObjectTypeQuery3") false 0 "ForDuration"))
        (if _returnvalue_3
          ;;[0.07292 0.07292 0.07292] 락온 시 컨트롤러 움직임으로 변경
          (Variables|Default|SetTarget%20Lock%20Actor (.HitActor (Collision|BreakHitResult _outhit)))
          (Variables|/Script/Engine.CharacterMovementComponent|SetbOrientRotationToMovement _charactermovement false)
          (Variables|/Script/Engine.CharacterMovementComponent|SetbUseControllerDesiredRotation _charactermovement true)
          ;;[0.07292 0.07292 0.07292] 락온 시 아이콘 생성
          (bind _returnvalue_4 (Game|SpawnActorfromClass "/Game/Blueprints/BP_TargetLockWidget.BP_TargetLockWidget_C" (Math|Transform|MakeTransform (Math|Vector|MakeVector (.x (.location (Transformation|GetActorTransform (Variables|Default|GetTarget%20Lock%20Actor)))) (.y (.location (Transformation|GetActorTransform (Variables|Default|GetTarget%20Lock%20Actor)))) (+ (.z (.location (Transformation|GetActorTransform (Variables|Default|GetTarget%20Lock%20Actor)))) 2e+01)) (.rotation (Transformation|GetActorTransform (Variables|Default|GetTarget%20Lock%20Actor))) "1.000000,1.000000,1.000000") "AlwaysSpawn" "MultiplyWithRoot" 0 0))
          (bind _output_get (Variables|Default|SetTarget%20Lock%20Widget _returnvalue_4))
          (Transformation|AttachActorToActor _output_get (Variables|Default|GetTarget%20Lock%20Actor) "None" "SnapToTarget" "SnapToTarget" "SnapToTarget" true))))))

(event Input|EnhancedActionEvents|EnhancedInputActionIA_Attack
  (params (ActionValue :type Boolean) (ElapsedSeconds :type Float%20%28double-precision%29) (TriggeredSeconds :type Float%20%28double-precision%29) (InputAction :type Input%20Action%20Object%20Reference :default "/Game/ThirdPerson/Input/Actions/IA_Attack.IA_Attack"))
  ;[0.05208 0.05208 0.05208] Sword Combo Animation
  (:Started
    (if (not (Variables|Default|GetisAttacking?))
      (Variables|Default|SetisAttacking? true)
      (Animation|Montage|PlayMontage (Variables|/Script/Engine.Character|GetMesh (Variables|Default|GetPlayer%20BP)) "/Game/Characters/Souls/combat/SwordAttackCombo_Montage.SwordAttackCombo_Montage"
        (:OnCompleted
          (Variables|Default|SetisAttacking? false :!label _label)
          (Variables|Default|Setcombo? false))
        (:OnInterrupted
          (goto _label))
        (:OnNotifyBegin
          (if (and (Variables|Default|GetisAttacking?) (Variables|Default|Getcombo?))
            (Variables|Default|Setcombo? false)
            (else
              (Animation|Montage|MontageStop (Components|SkeletalMesh|GetAnimInstance (Variables|/Script/Engine.Character|GetMesh (Variables|Default|GetPlayer%20BP))) 0.2 "/Game/Characters/Souls/combat/SwordAttackCombo_Montage.SwordAttackCombo_Montage")))))
      (else
        (Variables|Default|Setcombo? true)))))

(event Input|EnhancedActionEvents|EnhancedInputActionIA_Dodge
  (params (ActionValue :type Boolean) (ElapsedSeconds :type Float%20%28double-precision%29) (TriggeredSeconds :type Float%20%28double-precision%29) (InputAction :type Input%20Action%20Object%20Reference :default "/Game/ThirdPerson/Input/Actions/IA_Dodge.IA_Dodge"))
  (:Started
    (if (not (Variables|Default|GetisDodging?))
      (Variables|Default|SetisDodging? true)
      ;[0.05208 0.05208 0.05208] 닷지 연타해도 스팸 안되도록 방지
      (Utilities|FlowControl|Sequence
        (:then_0
          (if (Variables|/Script/Engine.CharacterMovementComponent|GetbUseControllerDesiredRotation (Variables|/Script/Engine.Character|GetCharacterMovement (Variables|Default|GetPlayer%20BP)))
            (switch string (Utilities|String|ToString(Text) (Class|KismetInputLibrary|KeyGetDisplayName (Variables|/Game/ThirdPerson/Blueprints/BP_ThirdPersonCharacter.BP_ThirdPersonCharacter_C|GetDirection%20Key (Variables|Default|GetPlayer%20BP)) true))
              (:W
                (Variables|Default|SetmovementDirection "NewEnumerator0"))
              (:A
                (Variables|Default|SetmovementDirection "NewEnumerator1"))
              (:S
                (Variables|Default|SetmovementDirection "NewEnumerator2"))
              (:D
                (Variables|Default|SetmovementDirection "NewEnumerator3")))
            (else
              (Variables|Default|SetmovementDirection "NewEnumerator0"))))
        (:then_1
          (Animation|Montage|PlayMontage (Variables|/Script/Engine.Character|GetMesh (Variables|Default|GetPlayer%20BP)) (Utilities|Select :Index (Variables|Default|GetmovementDirection) :NewEnumerator0 "/Game/Characters/Souls/combat/Dodge/Dodge_F_Montage.Dodge_F_Montage" :NewEnumerator1 "/Game/Characters/Souls/combat/Dodge/Dodge_L_Montage.Dodge_L_Montage" :NewEnumerator2 "/Game/Characters/Souls/combat/Dodge/Dodge_B_Montage.Dodge_B_Montage" :NewEnumerator3 "/Game/Characters/Souls/combat/Dodge/Dodge_R_Montage.Dodge_R_Montage")
            (:OnCompleted
              _)
            (:OnInterrupted
              _))
          (Variables|Default|SetisDodging? false))))))

(event EventTick
  (params (DeltaSeconds :type Float%20%28single-precision%29))
  (bind _player_bp (Variables|Default|GetPlayer%20BP))
  (bind _target_lock_actor (Variables|Default|GetTarget%20Lock%20Actor))
  (bind _returnvalue (Transformation|GetActorLocation _player_bp))
  (bind _returnvalue_2 (Transformation|GetActorLocation _target_lock_actor))
  (bind _returnvalue_3 (Math|Rotator|FindLookatRotation _returnvalue _returnvalue_2))
  ;[0.05208 0.05208 0.05208] Target Lock
  ;;[0.05208 0.05208 0.05208] Target Lock Update
  (Variables|Default|GetTarget%20Lock%20Actor
    (:then
      (Pawn|SetControlRotation (Pawn|GetController (Variables|Default|GetPlayer%20BP)) (Math|Rotator|MakeRotator (.roll _returnvalue_3) (+ (.pitch _returnvalue_3) -2e+01) (.yaw _returnvalue_3))))
    (:else)))

(event EventBeginPlay
  ;[0.05208 0.05208 0.05208] Get Player Class
  (bind _asbp_third_person_character (Utilities|Casting|CastToBP_ThirdPersonCharacter (Components|GetOwner)))
  (Variables|Default|SetPlayer%20BP _asbp_third_person_character))